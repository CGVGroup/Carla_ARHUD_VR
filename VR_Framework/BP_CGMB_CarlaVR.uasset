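; CARLA VR game mode for driving experiments with a Vivace vehicle in HUD or HDD variants.
; BeginPlay parses launch options for vehicle, user, scenario and session flags, then creates a GameLogger that records vehicle pose, inputs, controllers and camera every tick.
; Helpers spawn the vehicle at the scenario's spawn point and attach a VR pawn to a seat.
; Hand-tracking spawn, wheel calibration and settings menu logic are disconnected.
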(event EventBeginPlay
  (bind _optionsstring (Variables|Default|GetOptionsString))
  (bind _optionsstring_2 (Variables|Default|GetOptionsString))
  (bind _returnvalue (Class|GameplayStatics|ParseOption _optionsstring_2 "isStandalone"))
  (bind _returnvalue_2 (Class|GameplayStatics|ParseOption _optionsstring "isMultiplayer"))
  (bind _returnvalue_3 (Utilities|Enum|Equal(Enum) _returnvalue "true"))
  (bind _returnvalue_4 (Utilities|Enum|Equal(Enum) _returnvalue_2 "true"))
  (bind _output_get (Variables|Default|SetVehicleName (Class|GameplayStatics|ParseOption (Variables|Default|GetOptionsString) "VehicleName")))
  (if (Utilities|Enum|Equal(Enum) _output_get "BP_HUD_Vivace")
    (Variables|Default|SetVehicle%20VR "/Game/Carla/CarlaVR/VR_Framework/VR_Vehicles/VR_Vivace/BP_HUD_Vivace.BP_HUD_Vivace_C")
    (elif (Utilities|Enum|Equal(Enum) _output_get "BP_HDD_Vivace")
      (Variables|Default|SetVehicle%20VR "/Game/Carla/CarlaVR/VR_Framework/VR_Vehicles/VR_Vivace/BP_HDD_Vivace.BP_HDD_Vivace_C")
      (else
        (Development|PrintString "VR Vehicle not set" true true "(R=1.000000,G=0.027019,B=0.000000,A=1.000000)" 2e+01))))
  (Development|PrintString (Utilities|String|Append "Vehicle Name =" _output_get) true true "(R=0.000000,G=0.000000,B=1.000000,A=1.000000)" 2e+01)
  (Variables|Default|SetisPythonless _returnvalue_3)
  (Development|PrintString (Utilities|String|Append "is Pythonless =" (Utilities|String|ToString(Boolean) _returnvalue_3)) true true "(R=0.000000,G=0.000000,B=1.000000,A=1.000000)" 2e+01)
  (Variables|Default|SetisMultiplayer _returnvalue_4)
  (Development|PrintString (Utilities|String|Append "isMultiplayer" (Utilities|String|ToString(Boolean) _returnvalue_4)) true true "(R=0.000000,G=0.000000,B=1.000000,A=1.000000)" 2e+01)
  (Variables|Default|SetUserID (Class|GameplayStatics|ParseOption (Variables|Default|GetOptionsString) "UserID"))
  (Development|PrintString (Variables|Default|GetUserID) true true "(R=0.000000,G=1.000000,B=0.010844,A=1.000000)" 25.0)
  (bind _output_get_2 (Variables|Default|SetScenarioNumber (Class|GameplayStatics|ParseOption (Variables|Default|GetOptionsString) "ScenarioNumber")))
  (Development|PrintString _output_get_2 true true "(R=0.000000,G=0.660000,B=1.000000,A=1.000000)" 15.0)
  (bind _returnvalue_5 (Game|ConstructObjectfromClass "/Script/CarlaUnreal.GameLogger"))
  (bind _output_get_3 (Variables|Default|SetLogger _returnvalue_5))
  (Development|PrintString (Utilities|GetDisplayName _output_get_3))
  (Class|GameLogger|InitializeLogger _output_get_3 (Variables|Default|GetUserID) (Variables|Default|GetScenarioNumber) (Utilities|String|GetSubstring (Variables|Default|GetVehicleName) 3 3) "C:/ExperimentalMaterial"))

(event EventTick
  (params (DeltaSeconds :type Float%20%28single-precision%29))
  (bind _vrpawn_c (Variables|Default|GetVRPawn_C))
  (bind _targetvehicle (Variables|Default|GetTargetVehicle))
  (bind _returnvalue (Transformation|GetActorLocation _targetvehicle))
  (bind _returnvalue_2 (Transformation|GetActorRotation _targetvehicle))
  (bind _motioncontrollerleftgrip (Variables|/Game/Carla/CarlaVR/VR_Framework/Avatar/BP_P_VRPawn_Controller.BP_P_VRPawn_Controller_C|GetMotionControllerLeftGrip _vrpawn_c))
  (bind _motioncontrollerrightgrip (Variables|/Game/Carla/CarlaVR/VR_Framework/Avatar/BP_P_VRPawn_Controller.BP_P_VRPawn_Controller_C|GetMotionControllerRightGrip _vrpawn_c))
  (bind _camera (Variables|/Game/Carla/CarlaVR/VR_Framework/Avatar/BP_P_VRPawn_Controller.BP_P_VRPawn_Controller_C|GetCamera _vrpawn_c))
  (bind _vehiclemovementcomponent (Variables|/Script/ChaosVehicles.WheeledVehiclePawn|GetVehicleMovementComponent _targetvehicle))
  (bind _returnvalue_3 (Transformation|GetWorldLocation _motioncontrollerleftgrip))
  (bind _returnvalue_4 (Transformation|GetWorldLocation _motioncontrollerrightgrip))
  (bind _returnvalue_5 (Transformation|GetWorldLocation _camera))
  (bind _returnvalue_6 (Transformation|GetWorldRotation _camera))
  (Variables|Default|GetVRPawn_C
    (:then
      (bind _returnvalue_7 (Class|ChaosVehicleMovementComponent|GetThrottleInput _vehiclemovementcomponent))
      (bind _returnvalue_8 (Class|ChaosVehicleMovementComponent|GetSteeringInput _vehiclemovementcomponent))
      (bind _returnvalue_9 (Class|ChaosVehicleMovementComponent|GetBrakeInput _vehiclemovementcomponent))
      (Class|GameLogger|LogData (Variables|Default|GetLogger) (Utilities|String|Append "GM" "," (Utilities|String|ToString(Float) (Utilities|Time|GetGameTimeinSeconds)) "," (Utilities|String|Append (Utilities|String|ToString(Float) (.x _returnvalue)) "," (Utilities|String|ToString(Float) (.y _returnvalue)) "," (Utilities|String|ToString(Float) (.z _returnvalue)) "," (Utilities|String|ToString(Float) (.roll _returnvalue_2)) "," (Utilities|String|ToString(Float) (.pitch _returnvalue_2)) "," (Utilities|String|ToString(Float) (.yaw _returnvalue_2))) "," (Utilities|String|Append (Utilities|String|ToString(Float) _returnvalue_7) "," (Utilities|String|ToString(Float) _returnvalue_8) "," (Utilities|String|ToString(Float) _returnvalue_9)) "," (Utilities|String|Append (Utilities|String|ToString(Float) (.x _returnvalue_3)) "," (Utilities|String|ToString(Float) (.y _returnvalue_3)) "," (Utilities|String|ToString(Float) (.z _returnvalue_3)) "," (Utilities|String|ToString(Float) (.x _returnvalue_4)) "," (Utilities|String|ToString(Float) (.y _returnvalue_4)) "," (Utilities|String|ToString(Float) (.z _returnvalue_4)) "," (Utilities|String|ToString(Float) (.x _returnvalue_5)) "," (Utilities|String|ToString(Float) (.y _returnvalue_5)) "," (Utilities|String|ToString(Float) (.z _returnvalue_5)) ", " (Utilities|String|ToString(Float) (.roll _returnvalue_6)) "," (Utilities|String|ToString(Float) (.pitch _returnvalue_6)) "," (Utilities|String|ToString(Float) (.yaw _returnvalue_6))))))
    (:else)))

(fn ConstructionScript)

(fn FindRandomVehicleSpawn
  (bind _outactors (Actor|GetAllActorsOfClass "/Script/Carla.VehicleSpawnPoint"))
  (return (Utilities|Array|Get(acopy) _outactors (Math|Random|RandomIntegerinRange 0 (- (Utilities|Array|Length _outactors) 1)))))

(fn SpawnVehicleVR
  (params (VR_Vehicle :type Actor%20Class%20Reference))
  (bind _outactors (Actor|GetAllActorsOfClass "/Game/Carla/CarlaVR/VR_Framework/BP_VRVehicle_SpwanPoint.BP_VRVehicle_SpwanPoint_C"))
  (for _array_element _outactors
    (if (Utilities|Enum|Equal(Enum) (Variables|/Game/Carla/CarlaVR/VR_Framework/BP_VRVehicle_SpwanPoint.BP_VRVehicle_SpwanPoint_C|GetSpawnNumber _array_element) (Class|GameplayStatics|ParseOption (Variables|Default|GetOptionsString) "ScenarioNumber"))
      (switch string (Class|GameplayStatics|ParseOption (Variables|Default|GetOptionsString) "VehicleName")
        (:BP_HUD_Vivace
          (bind _returnvalue (Game|SpawnActorfromClass "/Game/Carla/CarlaVR/VR_Framework/VR_Vehicles/VR_Vivace/BP_HUD_Vivace.BP_HUD_Vivace_C" (Transformation|GetActorTransform _array_element) "AdjustIfPossibleButAlwaysSpawn" "MultiplyWithRoot" 0 0 0))
          (bind _asbase_vehicle_pawn (Utilities|Casting|CastToBaseVehiclePawn _returnvalue))
          (return _asbase_vehicle_pawn))
        (:BP_HDD_Vivace
          (bind _returnvalue_2 (Game|SpawnActorfromClass "/Game/Carla/CarlaVR/VR_Framework/VR_Vehicles/VR_Vivace/BP_HDD_Vivace.BP_HDD_Vivace_C" (Transformation|GetActorTransform _array_element) "AdjustIfPossibleButAlwaysSpawn" "MultiplyWithRoot" 0 0 0))
          (if (Class|HeadMountedDisplayFunctionLibrary|IsHeadMountedDisplayEnabled)
            _
            (else
              (bind _hdd (Default|GetHDD _returnvalue_2))
              (Transformation|SetActorScale3D _hdd "2.000000,2.000000,2.000000")
              (Transformation|AddLocalOffset (Variables|/Script/Engine.Actor|GetRootComponent _hdd) "-5.000000,0.000000,-2.000000" false false)
              (Transformation|SetWorldScale3D (Variables|/Game/Carla/CarlaVR/VR_Framework/VR_Vehicles/VR_Vivace/BP_HDD_Vivace.BP_HDD_Vivace_C|GetBP_DrivingSeat _returnvalue_2) "0, 0, 0")))
          (bind _asbase_vehicle_pawn_2 (Utilities|Casting|CastToBaseVehiclePawn _returnvalue_2))
          (return _asbase_vehicle_pawn_2)))
      (else
        (Development|PrintString "spawn number not found" true true "(R=0.000000,G=0.660000,B=1.000000,A=1.000000)" 1e+02))))
  (Development|PrintString (Utilities|String|Append (Utilities|String|ToString(Integer) (Utilities|Array|Length _outactors)) "spawn point found")))

(fn SpawnPawnObserver
  (params (PC%20Client :type Player%20Controller%20Object%20Reference))
  (bind _returnvalue (Game|SpawnActorfromClass "/Script/Engine.SpectatorPawn" (Math|Transform|MakeTransform "0.000000,0.000000,500.000000") "Undefined" "MultiplyWithRoot" 0 0))
  (Pawn|Possess PC%20Client _returnvalue))

(fn SpawnPawnVR
  (params (PlayerController :type Player%20Controller%20Object%20Reference))
  (bind _returnvalue (Pawn|GetControlledPawn PlayerController))
  (Utilities|IsValid _returnvalue
    (:Is%20Valid
      (Actor|DestroyActor _returnvalue))
    (:Is%20Not%20Valid
      _))
  (bind _returnvalue_2 (Game|SpawnActorfromClass "/Game/Carla/CarlaVR/VR_Framework/Avatar/BP_P_VRPawn_Controller.BP_P_VRPawn_Controller_C" (Math|Transform|MakeTransform "0, 0, 0") "AlwaysSpawn" "MultiplyWithRoot" 0 0))
  (if (not (Utilities|String|EndsWith (Variables|Default|GetUserID) "D"))
    _
    (else
      (Camera|SetFieldOfView (Variables|/Game/Carla/CarlaVR/VR_Framework/Avatar/BP_P_VRPawn_Controller.BP_P_VRPawn_Controller_C|GetCamera _returnvalue_2) 9e+01)
      (Class|SceneComponent|AddLocalTransform (Variables|/Game/Carla/CarlaVR/VR_Framework/Avatar/BP_P_VRPawn_Controller.BP_P_VRPawn_Controller_C|GetCamera _returnvalue_2) (Math|Transform|MakeTransform "8.000000,3.000000,5.000000" "-5.000000,0.000000,0.000000" "1.000000,1.000000,1.000000") false false)))
  (bind _output_get (Variables|Default|SetVRPawn_C _returnvalue_2))
  (Pawn|Possess PlayerController _output_get)
  (Development|PrintString "Spawn VRPawn" true true "(R=1.000000,G=0.007625,B=0.653255,A=1.000000)" 25.0)
  (return _output_get))

(fn SetupPlayerController
  (params (PC%20Client :type Player%20Controller%20Object%20Reference))
  (bind _output_get (Variables|Default|SetPlayerController PC%20Client))
  (Utilities|Casting|CastToBP_PC_CarlaVR _output_get
    (:then
      (bind _asbase_vehicle_pawn (CallFunction|SpawnVehicleVR (Variables|Default|GetVehicle%20VR)))
      (Variables|Default|SetTargetVehicle _asbase_vehicle_pawn))
    (:CastFailed
      (Development|PrintString "not a BP_PC_CarlaVR" true true "(R=1.000000,G=0.000000,B=0.096693,A=1.000000)" 25.0))))

(fn SetPlayerOnboard
  (bind _playercontroller (Variables|Default|GetPlayerController))
  (bind _targetvehicle (Variables|Default|GetTargetVehicle))
  (bind _spawn_location (CallFunction|GetVehicleSpawnPoints _targetvehicle (Variables|Default|GetSeat%20Position)))
  (bind _pawn (CallFunction|SpawnPawnVR _playercontroller))
  (CallFunction|AttachPlayer _pawn _targetvehicle _spawn_location)
  (CallFunction|SetPlayerControllerOnboardvehicle _playercontroller _targetvehicle)
  (bind _asbp_pc_carla_vr (Utilities|Casting|CastToBP_PC_CarlaVR _playercontroller))
  (Variables|/Game/Carla/CarlaVR/VR_Framework/BP_PC_CarlaVR.BP_PC_CarlaVR_C|SetisDriver _asbp_pc_carla_vr (Variables|Default|GetisDriver))
  (CameraFades|StartCameraFade :self (Game|GetPlayerCameraManager 0) :FromAlpha 1.0 :Duration 0.5))

(fn SetPlayerControllerOnboardvehicle
  (params (PlayerController :type Player%20Controller%20Object%20Reference) (Vehicle :type Base%20Vehicle%20Pawn%20Object%20Reference))
  (bind _asbp_pc_carla_vr (Utilities|Casting|CastToBP_PC_CarlaVR PlayerController)
    (:then
      (Default|SetonBoardVehicle _asbp_pc_carla_vr Vehicle))
    (:CastFailed
      (Development|PrintString "Not a BP_PC_CarlaVR controller" true true "(R=1.000000,G=0.000000,B=0.000000,A=1.000000)" 1e+01))))

(fn Deprecated--SetPawnOnboard
  (params (Pawn :type Actor%20Object%20Reference) (Vehicle :type Actor%20Object%20Reference)))

(fn AttachPlayer
  (params (Pawn :type Pawn%20Object%20Reference) (Vehicle :type Base%20Vehicle%20Pawn%20Object%20Reference) (SeatLocation :type Vector))
  (bind _returnvalue (Transformation|GetActorTransform Pawn))
  (Transformation|AttachActorToActor Pawn Vehicle "None" "KeepRelative" "KeepRelative" "KeepRelative" true)
  (Transformation|SetActorTransform Pawn (Math|Transform|MakeTransform SeatLocation (.rotation _returnvalue) (.scale _returnvalue))))

(fn GetVehicleSpawnPoints
  (params (Vehicle :type Base%20Vehicle%20Pawn%20Object%20Reference) (SeatPosition :type Integer))
  (bind _filteredarray (Utilities|Array|FilterArray (Actor|GetAllChildActors Vehicle true) "/Game/Carla/CarlaVR/VR_Framework/BP_VRSpawnPoint.BP_VRSpawnPoint_C"))
  (Variables|Default|SetisDriver (and (== (Math|Integer|%(Integer) SeatPosition (Utilities|Array|Length _filteredarray)) 0) (Variables|Default|GetisPythonless)))
  (if (Class|HeadMountedDisplayFunctionLibrary|IsHeadMountedDisplayEnabled)
    (return (.location (Transformation|GetActorTransform (Utilities|Array|Get(acopy) _filteredarray (Math|Integer|%(Integer) (Utilities|Array|Length _filteredarray) (+ SeatPosition 1))))))
    (else
      (return (.location (Transformation|GetActorTransform (Utilities|Array|Get(acopy) _filteredarray (Math|Integer|%(Integer) SeatPosition (Utilities|Array|Length _filteredarray)))))))))

(fn ChangeSeat
  (params (PlayerController :type Player%20Controller%20Object%20Reference) (Vehicle :type Base%20Vehicle%20Pawn%20Object%20Reference) (SeatPosition :type Integer))
  (bind _spawn_location (CallFunction|GetVehicleSpawnPoints Vehicle SeatPosition))
  (bind _pawn (CallFunction|SpawnPawnVR PlayerController))
  (CallFunction|AttachPlayer _pawn Vehicle _spawn_location)
  (bind _asbp_pc_carla_vr (Utilities|Casting|CastToBP_PC_CarlaVR PlayerController))
  (Variables|/Game/Carla/CarlaVR/VR_Framework/BP_PC_CarlaVR.BP_PC_CarlaVR_C|SetisDriver _asbp_pc_carla_vr (Variables|Default|GetisDriver)))

(fn CalibrateSteeringWheelRotation
  (params (ThumbPosition_L :type Vector) (ThumbPosition_R :type Vector)))

(fn SpawnSettingMenu)

(fn QuitCARLAVR
  (Game|QuitGame 0 "Quit" false))

(fn CalibrateSteeringWheelPosition
  (params (LThumb :type Vector)))

(fn MoveVRPawn
  (params (X :type Float%20%28double-precision%29) (Y :type Float%20%28double-precision%29) (Z :type Float%20%28double-precision%29) (RotZ :type Float%20%28double-precision%29))
  (bind _vrpawn_ht (Variables|Default|GetVRPawn_HT))
  (Utilities|IsValid _vrpawn_ht
    (:Is%20Valid
      (LocalVariables|SettargetPawn _vrpawn_ht))
    (:Is%20Not%20Valid
      (LocalVariables|SettargetPawn (Variables|Default|GetVRPawn_C))))
  (Transformation|AddActorLocalOffset (LocalVariables|GettargetPawn) (Math|Vector|MakeVector X Y Z) false false)
  (Transformation|AddActorLocalRotation (LocalVariables|GettargetPawn) (Math|Rotator|MakeRotator 0.0 0.0 RotZ) false false))