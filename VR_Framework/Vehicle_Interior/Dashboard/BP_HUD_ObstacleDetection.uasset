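; BP_HUD_ObstacleDetection is a VR vehicle dashboard Blueprint that detects objects overlapping its Box_Collider.
; Begin and end overlap events only print long-lived debug messages, with the begin message including the other actor's transform.
; Disconnected logic would cast the WBBHUD widget to W_BoundingBox and set an InRange flag, but it never runs, so overlaps do not update the HUD.
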(event OnComponentBeginOverlap(Box_Collider)
  (params (OverlappedComponent :type Primitive%20Component%20Object%20Reference) (OtherActor :type Actor%20Object%20Reference) (OtherComp :type Primitive%20Component%20Object%20Reference) (OtherBodyIndex :type Integer) (bFromSweep :type Boolean) (SweepResult :type Hit%20Result%20Structure%20%28by%20ref%29))
  (Development|PrintString (Utilities|String|Append "collision started with othe object at :" (Utilities|String|ToString(Transform) (Transformation|GetActorTransform OtherActor))) true true "(R=0.000000,G=0.660000,B=1.000000,A=1.000000)" 2e+01))

(event OnComponentEndOverlap(Box_Collider)
  (params (OverlappedComponent :type Primitive%20Component%20Object%20Reference) (OtherActor :type Actor%20Object%20Reference) (OtherComp :type Primitive%20Component%20Object%20Reference) (OtherBodyIndex :type Integer))
  (Development|PrintString "Collision ended" true true "(R=0.000000,G=0.660000,B=1.000000,A=1.000000)" 2e+01))

(fn ConstructionScript)