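; BP_DrivingSeat is the driving seat control rig in the VR vehicle interior, animating the steering wheel, pedals and gear shifter.
; Input events add scaled yaw deltas to the wheel and map throttle, brake and clutch values to absolute pedal rotations.
; The shifter combines Stick pitch and Shoulder roll to pose each gear and neutral.
; GetButtonPosition exposes world locations of two button-related components.
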(event Custom|Animate_SW
  (params (DeltaSteeringValue :type Float%20%28double-precision%29))
  ;[0.15 0.15 0.15 0.5] Transforms
  (Transformation|AddLocalRotation (Variables|Default|Getvivace_steering_wheel) (Math|Rotator|MakeRotator 0.0 0.0 (* DeltaSteeringValue 4.3e+02)) false false))

(event Custom|Animate_Throttle
  (params (ThrottleValue :type Float%20%28double-precision%29))
  ;[0.15 0.15 0.15 0.5] Transforms
  (Transformation|SetRelativeRotation (Variables|Default|Getvivace_pedal_gas) (Math|Rotator|MakeRotator (* ThrottleValue 35.0) 0.0 -9e+01) false false))

(event Custom|Animate_Brake
  (params (BrakeValue :type Float%20%28double-precision%29))
  ;[0.15 0.15 0.15 0.5] Transforms
  (Transformation|SetRelativeRotation (Variables|Default|Getvivace_pedal_brake_A) (Math|Rotator|MakeRotator (* BrakeValue 35.0) 0.0 -9e+01) false false))

(event Custom|Animate_Clutch
  (params (ClutchValue :type Float%20%28double-precision%29))
  ;[0.15 0.15 0.15 0.5] Transforms
  (Transformation|SetRelativeRotation (Variables|Default|Getvivace_pedal_clutch) (Math|Rotator|MakeRotator (* ClutchValue 35.0) 0.0 -9e+01) false false))

(event Custom|Animate_Gear
  (params (Gear :type Integer))
  (bind _shoulder (Variables|Default|GetShoulder))
  (bind _stick (Variables|Default|GetStick))
  ;[0.15 0.15 0.15 0.5] GearAniamtion
  (switch int Gear
    (:0
      (Transformation|SetRelativeRotation _stick "0, 0, 0" false false)
      (Transformation|SetRelativeRotation _shoulder "0, 0, 0" false false))
    (:1
      (Transformation|SetRelativeRotation _stick "-5.000000,0.000000,0.000000" false false)
      (Transformation|SetRelativeRotation _shoulder "0.000000,0.000000,10.000000" false false :!label _label))
    (:2
      (Transformation|SetRelativeRotation _stick "-5.000000,0.000000,0.000000" false false)
      (Transformation|SetRelativeRotation _shoulder "0.000000,0.000000,-10.000000" false false :!label _label_2))
    (:3
      (Transformation|SetRelativeRotation _stick "5.000000,0.000000,0.000000" false false)
      (goto _label))
    (:4
      (Transformation|SetRelativeRotation _stick "5.000000,0.000000,0.000000" false false)
      (goto _label_2))
    (:5
      (Transformation|SetRelativeRotation _stick "15.000000,0.000000,0.000000" false false)
      (goto _label))
    (:6
      (Transformation|SetRelativeRotation _stick "-15.000000,0.000000,0.000000" false false)
      (goto _label))))

(fn ConstructionScript)

(fn GetButtonPosition
  (return (Transformation|GetWorldLocation (Variables|Default|GetEndY)) (Transformation|GetWorldLocation (Variables|Default|GetButton_B))))