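; Player controller for CarlaVR that lets a VR user drive a Vivace vehicle with wheel, pedals and gear inputs.
; While IsDriver is on, Enhanced Input values go to the onboard HUD or HDD Vivace.
; SR_ events forward spawning, seat changes, pawn movement, calibration and settings to BP_CGMB_CarlaVR.
; A FANATEC device gets speed-scaled spring force feedback, and R aligns the headset to the vehicle's spawn point.
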(event Custom|SR_SpawnPlayer_VR
  ;[1 0.4745 0.07292] SR_SpawnPlayer
  (bind _asbp_cgmb_carla_vr (Utilities|Casting|CastToBP_CGMB_CarlaVR (Game|GetGameMode)))
  (Default|SetupPlayerController _asbp_cgmb_carla_vr self))

(event Custom|SR_ResetPawnCamera
  ;[0.8073 0.8073 0.8073 0.5] ResetPosition
  (bind _asbp_cgmb_carla_vr (Utilities|Casting|CastToBP_CGMB_CarlaVR (Game|GetGameMode)))
  (Default|CalibrateSteeringWheelRotation _asbp_cgmb_carla_vr "0, 0, 0" "0, 0, 0"))

(event Custom|CalibrateCamera
  (params (Start :type Vector) (Target :type Vector) (Pawn :type Pawn%20Object%20Reference))
  (Transformation|AddActorWorldOffset Pawn (- Target Start))
  (Class|HeadMountedDisplayFunctionLibrary|ResetOrientationandPosition 0.0 "OrientationAndPosition"))

(event Custom|SR_OpenSetting
  ;[0.15 0.15 0.15 0.5] OpenSetting
  (bind _asbp_cgmb_carla_vr (Utilities|Casting|CastToBP_CGMB_CarlaVR (Game|GetGameMode)))
  (Default|SpawnSettingMenu _asbp_cgmb_carla_vr))

(event Custom|SR_Change_Seat
  ;[1 1 1] Req_ChangingSeat
  (bind _asbp_cgmb_carla_vr (Utilities|Casting|CastToBP_CGMB_CarlaVR (Game|GetGameMode)))
  (Default|ChangeSeat _asbp_cgmb_carla_vr self (Variables|Default|GetOnBoardVehicle) (Variables|Default|GetSeatCounter)))

(event Custom|SR_CalibrateSWPosition
  (bind _asbp_cgmb_carla_vr (Utilities|Casting|CastToBP_CGMB_CarlaVR (Game|GetGameMode)))
  (Default|CalibrateSteeringWheelPosition _asbp_cgmb_carla_vr (Variables|Default|GetThumb_L)))

(event Custom|SR_CalibrateSWRotation
  ;[0.5541 0.5573 0.2844 0.5] SteeringWheel cAlibration
  (bind _asbp_cgmb_carla_vr (Utilities|Casting|CastToBP_CGMB_CarlaVR (Game|GetGameMode)))
  (if (and (Utilities|Operators|NotEqual(!=) :A (Variables|Default|GetThumb_R)) (Utilities|Operators|NotEqual(!=) :A (Variables|Default|GetThumb_L)))
    (Default|CalibrateSteeringWheelRotation _asbp_cgmb_carla_vr (Variables|Default|GetThumb_L) (Variables|Default|GetThumb_R))))

(event Custom|SR_MovePawn
  (params (X :type Float%20%28double-precision%29) (Y :type Float%20%28double-precision%29) (Z :type Float%20%28double-precision%29) (RotZ :type Float%20%28double-precision%29))
  (bind _asbp_cgmb_carla_vr (Utilities|Casting|CastToBP_CGMB_CarlaVR (Game|GetGameMode)))
  (Default|MoveVRPawn _asbp_cgmb_carla_vr X Y Z RotZ))

(event Custom|JoystickSubsystemReady
  ;[0.8827 0.0598 0.8906 0.5] Setting up joystick plugin
)

(event Custom|JoystickUnplugged
  (params (InstanceId :type Joystick%20Instance%20Id%20Structure%20%28by%20ref%29))
  ;[0.8827 0.0598 0.8906 0.5] Setting up joystick plugin
)

(event Custom|JoystickPluggedIn
  (params (InstanceId :type Joystick%20Instance%20Id%20Structure%20%28by%20ref%29))
  ;[0.8827 0.0598 0.8906 0.5] Setting up joystick plugin
)

(event Input|EnhancedActionEvents|EnhancedInputActionIA_PythonControl
  (params (ActionValue :type Boolean) (ElapsedSeconds :type Float%20%28double-precision%29) (TriggeredSeconds :type Float%20%28double-precision%29) (InputAction :type Input%20Action%20Object%20Reference :default "/Game/Carla/CarlaVR/VR_Framework/Avatar/Input/IA_PythonControl.IA_PythonControl"))
  ;[1 0.7042 0.09837] Toggle Pilot client
  (:Started
    (Variables|Default|SetisDriver (not (Variables|Default|GetisDriver)))))

(event Input|EnhancedActionEvents|EnhancedInputActionIA_ChangeSeat
  (params (ActionValue :type Boolean) (ElapsedSeconds :type Float%20%28double-precision%29) (TriggeredSeconds :type Float%20%28double-precision%29) (InputAction :type Input%20Action%20Object%20Reference :default "/Game/Carla/CarlaVR/VR_Framework/Avatar/Input/IA_ChangeSeat.IA_ChangeSeat"))
  ;[1 1 1] Req_ChangingSeat
  (:Started
    (if (Pawn|IsLocalPlayerController)
      (Math|Integer|IncrementInt (Variables|Default|GetSeatCounter)
        (:%20%20
          (CallFunction|SRChangeSeat))))))

(event Input|EnhancedActionEvents|EnhancedInputActionIA_Gear_2
  (params (ActionValue :type Boolean) (ElapsedSeconds :type Float%20%28double-precision%29) (TriggeredSeconds :type Float%20%28double-precision%29) (InputAction :type Input%20Action%20Object%20Reference :default "/Game/Carla/CarlaVR/VR_Framework/Avatar/Input/IA_Gear_2.IA_Gear_2"))
  (:Started
    (Variables|Default|SetGear 2)))

(event Input|EnhancedActionEvents|EnhancedInputActionIA_Gear_3
  (params (ActionValue :type Boolean) (ElapsedSeconds :type Float%20%28double-precision%29) (TriggeredSeconds :type Float%20%28double-precision%29) (InputAction :type Input%20Action%20Object%20Reference :default "/Game/Carla/CarlaVR/VR_Framework/Avatar/Input/IA_Gear_3.IA_Gear_3"))
  (:Started
    (Variables|Default|SetGear 3)))

(event Input|EnhancedActionEvents|EnhancedInputActionIA_Gear_4
  (params (ActionValue :type Boolean) (ElapsedSeconds :type Float%20%28double-precision%29) (TriggeredSeconds :type Float%20%28double-precision%29) (InputAction :type Input%20Action%20Object%20Reference :default "/Game/Carla/CarlaVR/VR_Framework/Avatar/Input/IA_Gear_4.IA_Gear_4"))
  (:Started
    (Variables|Default|SetGear 4)))

(event Input|EnhancedActionEvents|EnhancedInputActionIA_Gear_6
  (params (ActionValue :type Boolean) (ElapsedSeconds :type Float%20%28double-precision%29) (TriggeredSeconds :type Float%20%28double-precision%29) (InputAction :type Input%20Action%20Object%20Reference :default "/Game/Carla/CarlaVR/VR_Framework/Avatar/Input/IA_Gear_6.IA_Gear_6"))
  (:Started
    (Variables|Default|SetGear 6)))

(event Input|EnhancedActionEvents|EnhancedInputActionIA_Gear_5
  (params (ActionValue :type Boolean) (ElapsedSeconds :type Float%20%28double-precision%29) (TriggeredSeconds :type Float%20%28double-precision%29) (InputAction :type Input%20Action%20Object%20Reference :default "/Game/Carla/CarlaVR/VR_Framework/Avatar/Input/IA_Gear_5.IA_Gear_5"))
  (:Started
    (Variables|Default|SetGear 5)))

(event Input|EnhancedActionEvents|EnhancedInputActionIA_Throttle
  (params (ActionValue :type Float%20%28double-precision%29) (ElapsedSeconds :type Float%20%28double-precision%29) (TriggeredSeconds :type Float%20%28double-precision%29) (InputAction :type Input%20Action%20Object%20Reference :default "/Game/Carla/CarlaVR/VR_Framework/Avatar/Input/IA_Throttle.IA_Throttle"))
  (bind _isdriver (Variables|Default|GetisDriver))
  (bind _onboardvehicle (Variables|Default|GetOnBoardVehicle))
  ;[0.3046 0.5781 0.05406] Throttle
  (:Triggered
    (Variables|Default|SetThrottle (* (- 1.0 (Variables|Default|GetClutch)) (Math|Float|MapRangeClamped ActionValue 1.0 -1.0 0.0 1.0)) :!label _label)
    (if _isdriver :!label _label_2
      (Utilities|IsValid _onboardvehicle
        (:Is%20Valid
          (bind _asbp_hud_vivace (Utilities|Casting|CastToBP_HUD_Vivace _onboardvehicle)
            (:then
              (Default|SetCustomThrottle _asbp_hud_vivace (Variables|Default|GetThrottle)))
            (:CastFailed
              (bind _asbp_hdd_vivace (Utilities|Casting|CastToBP_HDD_Vivace _onboardvehicle))
              (Default|SetCustomThrottle _asbp_hdd_vivace (Variables|Default|GetThrottle))))
          (Development|PrintString (Utilities|String|Append "Throttle = " (Utilities|String|ToString(Float) (Variables|Default|GetThrottle)) "   is Driver is  " (Utilities|String|ToString(Boolean) _isdriver)) true true "(R=0.000000,G=0.660000,B=1.000000,A=1.000000)" 0.01)))))
  (:Ongoing
    (goto _label))
  (:Canceled
    (Variables|Default|SetThrottle 0.0 :!label _label_3)
    (goto _label_2))
  (:Completed
    (goto _label_3)))

(event Input|EnhancedActionEvents|EnhancedInputActionIA_Settings
  (params (ActionValue :type Boolean) (ElapsedSeconds :type Float%20%28double-precision%29) (TriggeredSeconds :type Float%20%28double-precision%29) (InputAction :type Input%20Action%20Object%20Reference :default "/Game/Carla/CarlaVR/VR_Framework/Avatar/Input/IA_Settings.IA_Settings"))
  ;[0.15 0.15 0.15 0.5] OpenSetting
  (:Started
    (CallFunction|SROpenSetting)))

(event Input|EnhancedActionEvents|EnhancedInputActionIA_Clutch
  (params (ActionValue :type Float%20%28double-precision%29) (ElapsedSeconds :type Float%20%28double-precision%29) (TriggeredSeconds :type Float%20%28double-precision%29) (InputAction :type Input%20Action%20Object%20Reference :default "/Game/Carla/CarlaVR/VR_Framework/Avatar/Input/IA_Clutch.IA_Clutch"))
  (bind _onboardvehicle (Variables|Default|GetOnBoardVehicle))
  ;[0.1979 0.3594 0.07113 0.5] Clutch
  (:Triggered
    (Variables|Default|SetClutch (Math|Float|MapRangeClamped ActionValue 1.0 -1.0 0.0 1.0))
    (Development|PrintString (Utilities|String|Append "Clutch = " (Utilities|String|ToString(Float) (Variables|Default|GetClutch))) true true "(R=0.000000,G=0.660000,B=1.000000,A=1.000000)" 0.01 :!label _label)
    (Utilities|IsValid _onboardvehicle
      (:Is%20Valid
        (bind _asbp_hud_vivace (Utilities|Casting|CastToBP_HUD_Vivace _onboardvehicle)
          (:then
            (if (> (Variables|Default|GetClutch) 0.5)
              (Class|CarlaWheeledVehicle|ToggleReverse _asbp_hud_vivace)))
          (:CastFailed
            (bind _asbp_hdd_vivace (Utilities|Casting|CastToBP_HDD_Vivace _onboardvehicle))
            (if (> (Variables|Default|GetClutch) 0.5)
              (Class|CarlaWheeledVehicle|ToggleReverse _asbp_hdd_vivace)))))))
  (:Completed
    (Variables|Default|SetClutch 0.0)
    (goto _label)))

(event Input|EnhancedActionEvents|EnhancedInputActionIA_CalibrateSteeringWheel_R
  (params (ActionValue :type Boolean) (ElapsedSeconds :type Float%20%28double-precision%29) (TriggeredSeconds :type Float%20%28double-precision%29) (InputAction :type Input%20Action%20Object%20Reference :default "/Game/Carla/CarlaVR/VR_Framework/Avatar/Input/IA_CalibrateSteeringWheel_R.IA_CalibrateSteeringWheel_R"))
  ;[0.5541 0.5573 0.2844 0.5] SteeringWheel cAlibration
  (:Canceled
    (Variables|Default|SetisRPressed false :!label _label))
  (:Completed
    (goto _label)))

(event Input|EnhancedActionEvents|EnhancedInputActionIA_CalibrateSteeringWheel_L
  (params (ActionValue :type Boolean) (ElapsedSeconds :type Float%20%28double-precision%29) (TriggeredSeconds :type Float%20%28double-precision%29) (InputAction :type Input%20Action%20Object%20Reference :default "/Game/Carla/CarlaVR/VR_Framework/Avatar/Input/IA_CalibrateSteeringWheel_L.IA_CalibrateSteeringWheel_L"))
  (:Canceled
    (Variables|Default|SetisLPressed false :!label _label))
  (:Completed
    (goto _label)))

(event Input|EnhancedActionEvents|EnhancedInputActionIA_ResetPawnCamera
  (params (ActionValue :type Boolean) (ElapsedSeconds :type Float%20%28double-precision%29) (TriggeredSeconds :type Float%20%28double-precision%29) (InputAction :type Input%20Action%20Object%20Reference :default "/Game/Carla/CarlaVR/VR_Framework/Avatar/Input/IA_ResetPawnCamera.IA_ResetPawnCamera"))
  ;[0.8073 0.8073 0.8073 0.5] ResetPosition
  (:Started
    (CallFunction|SRResetPawnCamera)))

(event Input|EnhancedActionEvents|EnhancedInputActionIA_MovePawn_X
  (params (ActionValue :type Float%20%28double-precision%29) (ElapsedSeconds :type Float%20%28double-precision%29) (TriggeredSeconds :type Float%20%28double-precision%29) (InputAction :type Input%20Action%20Object%20Reference :default "/Game/Carla/CarlaVR/VR_Framework/Avatar/Input/IA_MovePawn_X.IA_MovePawn_X"))
  (CallFunction|SRMovePawn ActionValue 0.0 0.0 0.0))

(event Input|EnhancedActionEvents|EnhancedInputActionIA_MovePawn_Y
  (params (ActionValue :type Float%20%28double-precision%29) (ElapsedSeconds :type Float%20%28double-precision%29) (TriggeredSeconds :type Float%20%28double-precision%29) (InputAction :type Input%20Action%20Object%20Reference :default "/Game/Carla/CarlaVR/VR_Framework/Avatar/Input/IA_MovePawn_Y.IA_MovePawn_Y"))
  (CallFunction|SRMovePawn 0.0 ActionValue 0.0 0.0))

(event Input|EnhancedActionEvents|EnhancedInputActionIA_MovePawn_Z
  (params (ActionValue :type Float%20%28double-precision%29) (ElapsedSeconds :type Float%20%28double-precision%29) (TriggeredSeconds :type Float%20%28double-precision%29) (InputAction :type Input%20Action%20Object%20Reference :default "/Game/Carla/CarlaVR/VR_Framework/Avatar/Input/IA_MovePawn_Z.IA_MovePawn_Z"))
  (CallFunction|SRMovePawn 0.0 0.0 ActionValue 0.0))

(event Input|EnhancedActionEvents|EnhancedInputActionIA_Steering
  (params (ActionValue :type Float%20%28double-precision%29) (ElapsedSeconds :type Float%20%28double-precision%29) (TriggeredSeconds :type Float%20%28double-precision%29) (InputAction :type Input%20Action%20Object%20Reference :default "/Game/Carla/CarlaVR/VR_Framework/Avatar/Input/IA_Steering.IA_Steering"))
  (bind _onboardvehicle (Variables|Default|GetOnBoardVehicle))
  (bind _onboardvehicle_2 (Variables|Default|GetOnBoardVehicle))
  (bind _vehiclemovementcomponent (Variables|/Script/ChaosVehicles.WheeledVehiclePawn|GetVehicleMovementComponent _onboardvehicle))
  (bind _returnvalue (Vehicle|GetForwardSpeed _vehiclemovementcomponent))
  (bind _returnvalue_2 (/ _returnvalue 3.9e+03))
  (bind _returnvalue_3 (Math|Float|Min(Float) _returnvalue_2 1.0))
  (bind _returnvalue_4 (Math|Conversions|ToVector(Float) _returnvalue_3))
  ;[0.3046 0.5781 0.05406] Steering
  (:Triggered
    (Variables|Default|SetSteering ActionValue :!label _label)
    (if (Variables|Default|GetisDriver) :!label _label_2
      (Utilities|IsValid _onboardvehicle_2
        (:Is%20Valid
          (bind _asbp_hud_vivace (Utilities|Casting|CastToBP_HUD_Vivace _onboardvehicle_2)
            (:then
              (Default|SetCustomSteering _asbp_hud_vivace (Variables|Default|GetSteering)))
            (:CastFailed
              (bind _asbp_hdd_vivace (Utilities|Casting|CastToBP_HDD_Vivace _onboardvehicle_2))
              (Default|SetCustomSteering _asbp_hdd_vivace (Variables|Default|GetSteering))))
          (Development|PrintString (Utilities|String|Append "Steering = " (Utilities|String|ToString(Float) (Variables|Default|GetSteering))) true true "(R=0.000000,G=0.660000,B=1.000000,A=1.000000)" 0.01)
          ;[0.01123 0.15 0.132 0.5] FFB
          (bind _ffb_effect (Variables|Default|GetFFB_Effect)
            (:then
              (Variables|/Script/JoystickPlugin.ForceFeedbackEffectCondition|SetEffectData _ffb_effect (Utilities|Struct|MakeForceFeedbackEffectConditionData "(DirectionType=Cartesian,Direction=(X=0.000000,Y=0.000000,Z=0.000000))" (Utilities|Struct|MakeForceFeedbackEffectDurationData 1.0 true) "(Delay=0.000000,RetriggerDelay=0.000000)" "Spring" _returnvalue_4 _returnvalue_4 _returnvalue_4 _returnvalue_4 "0.000000,0.000000,0.000000" "0.000000,0.000000,0.000000"))
              (Class|ForceFeedbackEffectBase|UpdateEffect (Variables|Default|GetFFB_Effect)))
            (:else))))))
  (:Ongoing
    (goto _label))
  (:Canceled
    (Variables|Default|SetSteering 0.0 :!label _label_3)
    (goto _label_2))
  (:Completed
    (goto _label_3)))

(event Input|EnhancedActionEvents|EnhancedInputActionIA_Brake
  (params (ActionValue :type Float%20%28double-precision%29) (ElapsedSeconds :type Float%20%28double-precision%29) (TriggeredSeconds :type Float%20%28double-precision%29) (InputAction :type Input%20Action%20Object%20Reference :default "/Game/Carla/CarlaVR/VR_Framework/Avatar/Input/IA_Brake.IA_Brake"))
  (bind _onboardvehicle (Variables|Default|GetOnBoardVehicle))
  ;[0.3046 0.5781 0.05406] Braking
  (:Triggered
    (Variables|Default|SetBrake (Math|Float|MapRangeClamped ActionValue 1.0 -1.0 0.0 1.0) :!label _label)
    (if (Variables|Default|GetisDriver) :!label _label_2
      (Utilities|IsValid _onboardvehicle
        (:Is%20Valid
          (bind _asbp_hud_vivace (Utilities|Casting|CastToBP_HUD_Vivace _onboardvehicle)
            (:then
              (Default|SetCustomBrake _asbp_hud_vivace (Variables|Default|GetBrake)))
            (:CastFailed
              (bind _asbp_hdd_vivace (Utilities|Casting|CastToBP_HDD_Vivace _onboardvehicle))
              (Default|SetCustomBrake _asbp_hdd_vivace (Variables|Default|GetBrake))))
          (Development|PrintString (Utilities|String|Append "Braking = " (Utilities|String|ToString(Float) (Variables|Default|GetBrake))) true true "(R=0.000000,G=0.660000,B=1.000000,A=1.000000)" 0.01)))))
  (:Ongoing
    (goto _label))
  (:Canceled
    (Variables|Default|SetBrake 0.0 :!label _label_3)
    (goto _label_2))
  (:Completed
    (goto _label_3)))

(event Input|EnhancedActionEvents|EnhancedInputActionIA_ParkBrake
  (params (ActionValue :type Boolean) (ElapsedSeconds :type Float%20%28double-precision%29) (TriggeredSeconds :type Float%20%28double-precision%29) (InputAction :type Input%20Action%20Object%20Reference :default "/Game/Carla/CarlaVR/VR_Framework/Avatar/Input/IA_ParkBrake.IA_ParkBrake"))
  (bind _onboardvehicle (Variables|Default|GetOnBoardVehicle))
  ;[0.3046 0.5781 0.05406] HandBrake
  (:Started
    (Variables|Default|SetHand%20Brake true)
    (if (Variables|Default|GetisDriver) :!label _label
      (Utilities|IsValid _onboardvehicle
        (:Is%20Valid
          (bind _asbp_vr_vivace (Utilities|Casting|CastToBP_VR_Vivace _onboardvehicle))
          (Development|PrintString (Utilities|String|Append "Handbrake is = " (Utilities|String|ToString(Boolean) (Variables|Default|GetHand%20Brake))))
          (Default|SetCustomHandBrake _asbp_vr_vivace (Variables|Default|GetHand%20Brake))))))
  (:Canceled
    (Variables|Default|SetHand%20Brake false)
    (goto _label)))

(event Input|EnhancedActionEvents|EnhancedInputActionIA_Quit
  (params (ActionValue :type Boolean) (ElapsedSeconds :type Float%20%28double-precision%29) (TriggeredSeconds :type Float%20%28double-precision%29) (InputAction :type Input%20Action%20Object%20Reference :default "/Game/Carla/CarlaVR/VR_Framework/Avatar/Input/IA_Quit.IA_Quit"))
  (Game|QuitGame 0 "Quit" false))

(event Input|EnhancedActionEvents|EnhancedInputActionIA_RotatePawn
  (params (ActionValue :type Float%20%28double-precision%29) (ElapsedSeconds :type Float%20%28double-precision%29) (TriggeredSeconds :type Float%20%28double-precision%29) (InputAction :type Input%20Action%20Object%20Reference :default "/Game/Carla/CarlaVR/VR_Framework/Avatar/Input/IA_RotatePawn.IA_RotatePawn"))
  (CallFunction|SRMovePawn 0.0 0.0 0.0 ActionValue))

(event Input|EnhancedActionEvents|EnhancedInputActionIA_Gear_R
  (params (ActionValue :type Boolean) (ElapsedSeconds :type Float%20%28double-precision%29) (TriggeredSeconds :type Float%20%28double-precision%29) (InputAction :type Input%20Action%20Object%20Reference :default "/Game/Carla/CarlaVR/VR_Framework/Avatar/Input/IA_Gear_R.IA_Gear_R"))
  (bind _onboardvehicle (Variables|Default|GetOnBoardVehicle))
  ;[0.3046 0.5781 0.05406] Reverse
  (:Started
    (Class|CarlaWheeledVehicle|SetReverse (Variables|Default|GetOnBoardVehicle) true))
  (:Completed
    ;[0.4238 1 0 0.5] Gear selection
    (Variables|Default|SetGear 0)
    (if (Variables|Default|GetisDriver)
      (Variables|Default|SetReverse (not (Variables|Default|GetReverse)))
      (Utilities|IsValid _onboardvehicle
        (:Is%20Valid
          (bind _asbp_vr_vivace (Utilities|Casting|CastToBP_VR_Vivace _onboardvehicle))
          (Development|PrintString (Utilities|String|Append "Gear is = " (Utilities|String|ToString(Integer) (Variables|Default|GetGear))) true true "(R=0.000000,G=0.660000,B=1.000000,A=1.000000)" 0.01)
          (Default|SetCustomGear _asbp_vr_vivace (Variables|Default|GetGear)))))))

(event Input|EnhancedActionEvents|EnhancedInputActionIA_Gear_1
  (params (ActionValue :type Boolean) (ElapsedSeconds :type Float%20%28double-precision%29) (TriggeredSeconds :type Float%20%28double-precision%29) (InputAction :type Input%20Action%20Object%20Reference :default "/Game/Carla/CarlaVR/VR_Framework/Avatar/Input/IA_Gear_1.IA_Gear_1"))
  (bind _onboardvehicle (Variables|Default|GetOnBoardVehicle))
  ;[0.4238 1 0 0.5] Gear selection
  (:Started
    (Class|CarlaWheeledVehicle|SetReverse (Variables|Default|GetOnBoardVehicle) false)
    (Variables|Default|SetGear 1)
    (if (Variables|Default|GetisDriver) :!label _label
      (Variables|Default|SetReverse (not (Variables|Default|GetReverse)))
      (Utilities|IsValid _onboardvehicle
        (:Is%20Valid
          (bind _asbp_vr_vivace (Utilities|Casting|CastToBP_VR_Vivace _onboardvehicle))
          (Development|PrintString (Utilities|String|Append "Gear is = " (Utilities|String|ToString(Integer) (Variables|Default|GetGear))) true true "(R=0.000000,G=0.660000,B=1.000000,A=1.000000)" 0.01)
          (Default|SetCustomGear _asbp_vr_vivace (Variables|Default|GetGear))))))
  (:Completed
    (Variables|Default|SetGear 0)
    (goto _label)))

(event EventBeginPlay
  (bind _returnvalue (|JoystickSubsystem))
  (bind _ffb_effect (Variables|Default|GetFFB_effect))
  ;[1 1 1] Request Spawning Player
  (if (Pawn|IsLocalPlayerController)
    (CallFunction|SRSpawnPlayerVR)
    (Input|AddMappingContext (PlayerController|LocalPlayerSubsystems|GetEnhancedInputLocalPlayerSubsystem) "/Game/Carla/CarlaVR/VR_Framework/Avatar/Input/IMC_CarlaVR.IMC_CarlaVR" 0 "(bIgnoreAllPressedKeysUntilRelease=True,bForceImmediately=False,bNotifyUserSettings=False)")
    ;[0.8827 0.0598 0.8906 0.5] Setting up joystick plugin
    (EventDispatchers|AssignJoystickSubsystemReady _returnvalue (delegate Custom|JoystickSubsystemReady))
    (EventDispatchers|BindEventtoJoystickPluggedinDelegate _returnvalue (delegate Custom|JoystickPluggedIn))
    (EventDispatchers|BindEventtoJoystickUnpluggedDelegate _returnvalue (delegate Custom|JoystickUnplugged))
    ;;[0.8906 0.1093 0.664 0.5] Select controller
    (for _array_element (Class|JoystickSubsystem|GetInstanceIds _returnvalue)
      (bind _joystickinfo (Class|JoystickSubsystem|GetJoystickInfo (|JoystickSubsystem) _array_element))
      (if (Utilities|String|StartsWith (.DeviceName (Utilities|Struct|BreakJoystickInformation _joystickinfo)) "FANATEC")
        (Variables|Default|SetDeviceID (.InstanceId (Utilities|Struct|BreakJoystickInformation _joystickinfo)))
        ;;[0.6146 0.01948 0.4182 0.5] FF init
        (bind _returnvalue_2 (Game|ConstructObjectfromClass "/Game/Carla/CarlaVR/VR_Framework/Avatar/Input/FF_Condition_Steering.FF_Condition_Steering_C" (Variables|Default|GetDeviceID)))
        (Variables|Default|SetFFB_Effect _returnvalue_2)
        (Class|ForceFeedbackEffectBase|InitialiseEffect _ffb_effect)
        (Class|ForceFeedbackEffectBase|StartEffect _ffb_effect)))))

(event Input|AxisEvents|InputAxisMoveForward
  (params (AxisValue :type Float%20%28single-precision%29))
  ;[0.3046 0.5781 0.05406] Throttle
)

(event Input|AxisEvents|InputAxisBrake
  (params (AxisValue :type Float%20%28single-precision%29))
  ;[0.3046 0.5781 0.05406] Braking
)

(event Input|KeyboardEvents|R
  (params (Key :type Key%20Structure :default "None"))
  (bind _onboardvehicle (Variables|Default|GetOnBoardVehicle))
  (:Pressed
    (bind _asbp_p_vrpawn_controller (Utilities|Casting|CastToBP_P_VRPawn_Controller (Game|Player|GetPlayerPawn 0)))
    (bind _asbp_hdd_vivace (Utilities|Casting|CastToBP_HDD_Vivace _onboardvehicle)
      (:then
        (CallFunction|CalibrateCamera (Transformation|GetWorldLocation (Variables|/Game/Carla/CarlaVR/VR_Framework/Avatar/BP_P_VRPawn_Controller.BP_P_VRPawn_Controller_C|GetHeadMountedDisplayMesh _asbp_p_vrpawn_controller)) (Transformation|GetWorldLocation (Variables|/Game/Carla/CarlaVR/VR_Framework/VR_Vehicles/VR_Vivace/BP_HDD_Vivace.BP_HDD_Vivace_C|GetBP_VRSpawnPoint1 _asbp_hdd_vivace)) _asbp_p_vrpawn_controller))
      (:CastFailed
        (bind _asbp_hud_vivace (Utilities|Casting|CastToBP_HUD_Vivace _onboardvehicle))
        (CallFunction|CalibrateCamera (Transformation|GetWorldLocation (Variables|/Game/Carla/CarlaVR/VR_Framework/Avatar/BP_P_VRPawn_Controller.BP_P_VRPawn_Controller_C|GetHeadMountedDisplayMesh _asbp_p_vrpawn_controller)) (Transformation|GetWorldLocation (Variables|/Game/Carla/CarlaVR/VR_Framework/VR_Vehicles/VR_Vivace/BP_HUD_Vivace.BP_HUD_Vivace_C|GetBP_VRSpawnPoint1 _asbp_hud_vivace)) _asbp_p_vrpawn_controller)))))

(fn ConstructionScript)

(fn SetonBoardVehicle
  (params (vehicle :type Base%20Vehicle%20Pawn%20Object%20Reference))
  (bind _output_get (Variables|Default|SetOnBoardVehicle vehicle))
  (Development|PrintString (Utilities|String|Append "OnBoardVehicle is = " (Utilities|GetDisplayName _output_get)) true true "(R=0.000000,G=0.660000,B=1.000000,A=1.000000)" 4e+01))

(fn ToggleMenu
  (params (bActiveMenuHandRight :type Boolean)))