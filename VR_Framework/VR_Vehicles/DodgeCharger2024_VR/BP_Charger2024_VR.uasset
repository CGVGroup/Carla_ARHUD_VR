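; VR-drivable 2024 Dodge Charger vehicle Blueprint for the CarlaVR game mode.
; BeginPlay registers the car as the game mode's target vehicle, boards the player after a delay, and links the speedometer and RPM widgets to it.
; It also binds joystick plugin delegates and constructs a steering force-feedback effect for the first device.
; Custom events pass throttle, steering, brake, handbrake, reverse and gear commands to the vehicle.
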(event Custom|Set_Custom_Gear
  (params (Gear :type Integer))
  (Class|ChaosVehicleMovementComponent|SetTargetGear (Variables|Default|GetVehicleMovementComponent self) Gear true))

(event Custom|Set_Custom_Throttle
  (params (throttle :type Float%20%28double-precision%29))
  ;[0.591 0.8125 0.2236] Throttle
  (Class|CarlaWheeledVehicle|SetThrottleInput throttle))

(event Custom|SR_Spawn_Occupant
  ;[1 0.6806 0.08897] SR_SpawnOwningPlayer
  (bind _asbp_cgmb_carla_vr (Utilities|Casting|CastToBP_CGMB_CarlaVR (Game|GetGameMode)))
  (Variables|/Game/Carla/CarlaVR/VR_Framework/BP_CGMB_CarlaVR.BP_CGMB_CarlaVR_C|SetTargetVehicle _asbp_cgmb_carla_vr self)
  (Utilities|FlowControl|Delay 3.0)
  (Default|SetPlayerOnboard _asbp_cgmb_carla_vr))

(event Custom|Set_Custom_Steering
  (params (Steering :type Float%20%28double-precision%29))
  ;[0.591 0.8125 0.2236] Steering
  (Class|CarlaWheeledVehicle|SetSteeringInput Steering))

(event Custom|Set_Custom_Brake
  (params (Brake :type Float%20%28double-precision%29))
  ;[0.591 0.8125 0.2236] Brake
  (Class|CarlaWheeledVehicle|SetBrakeInput Brake))

(event Custom|Set_Custom_HandBrake
  (params (HandBrake :type Boolean))
  ;[0.5906 0.8148 0.2232] HandBrake
  (Class|CarlaWheeledVehicle|SetHandbrakeInput HandBrake))

(event Custom|Set_Custom_Reverse
  (params (Reverse :type Boolean))
  ;[0.5906 0.8148 0.2232] Reverse
  (Class|CarlaWheeledVehicle|SetReverse Reverse))

(event Custom|JoystickSubsystemReady
  ;[0.15 0.15 0.15 0.5] Setting up joystick plugin
  (Development|PrintString "Joystick subsystem is ready" true true "(R=0.000000,G=0.966856,B=1.000000,A=1.000000)" 5.0))

(event Custom|JoystickUnplugged
  (params (InstanceId :type Joystick%20Instance%20Id%20Structure%20%28by%20ref%29))
  ;[0.15 0.15 0.15 0.5] Setting up joystick plugin
)

(event Custom|JoystickPluggedIn
  (params (InstanceId :type Joystick%20Instance%20Id%20Structure%20%28by%20ref%29))
  ;[0.15 0.15 0.15 0.5] Setting up joystick plugin
)

(event EventBeginPlay
  (bind _returnvalue (|JoystickSubsystem))
  ;[1 1 1] Find Self
  (|CallParentFunction)
  (CallFunction|SRSpawnOccupant)
  (bind _aswb_speedometer (Utilities|Casting|CastToWB_Speedometer (UserInterface|GetUserWidgetObject (Variables|Default|GetW_Speedometer))))
  (Default|SetParentVehicle _aswb_speedometer self)
  (bind _aswb_rpm (Utilities|Casting|CastToWB_RPM (UserInterface|GetUserWidgetObject (Variables|Default|GetW_RPM))))
  (Default|SetParentVehicle _aswb_rpm self)
  ;[0.15 0.15 0.15 0.5] Setting up joystick plugin
  (EventDispatchers|AssignJoystickSubsystemReady _returnvalue (delegate Custom|JoystickSubsystemReady))
  (EventDispatchers|BindEventtoJoystickPluggedinDelegate _returnvalue (delegate Custom|JoystickPluggedIn))
  (EventDispatchers|BindEventtoJoystickUnpluggedDelegate _returnvalue (delegate Custom|JoystickUnplugged))
  (Variables|Default|SetDeviceID (Utilities|Array|Get(acopy) (Class|JoystickSubsystem|GetInstanceIds _returnvalue)))
  (bind _returnvalue_2 (Game|ConstructObjectfromClass "/Game/Carla/CarlaVR/VR_Framework/Avatar/Input/FF_Condition_Steering.FF_Condition_Steering_C" (Variables|Default|GetDeviceID)))
  (Variables|Default|SetFFB_Effect _returnvalue_2))

(event Collision|EventActorBeginOverlap
  (params (OtherActor :type Actor%20Object%20Reference)))

(fn ConstructionScript
  (|CallParentFunction))