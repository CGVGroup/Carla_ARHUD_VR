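; Drivable Vivace vehicle for Carla VR, with speedometer and RPM widgets, that boards the player via the game mode after a delay.
; Custom input events drive Chaos throttle, steering, brake and handbrake and animate the driving seat; clutch and gear only animate or store values.
; BeginPlay creates a steering force-feedback effect through the joystick plugin.
; Tick feeds engine and wind audio, while forced manual-gear and RPM-calculation logic sits disconnected.
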(event Custom|Set_Custom_Throttle
  (params (throttle :type Float%20%28double-precision%29))
  ;[0.02062 0.15 0.03603 0.5] Controls
  (bind _aschaos_wheeled_vehicle_movement_component (Utilities|Casting|CastToChaosWheeledVehicleMovementComponent (Variables|Default|GetVehicleMovementComponent)))
  (Class|ChaosVehicleMovementComponent|SetThrottleInput _aschaos_wheeled_vehicle_movement_component throttle)
  (bind _asbp_driving_seat (Utilities|Casting|CastToBP_DrivingSeat (Variables|/Script/Engine.ChildActorComponent|GetChildActor (Variables|Default|GetBP_DrivingSeat))))
  (Default|AnimateThrottle _asbp_driving_seat throttle))

(event Custom|Set_Custom_Clutch
  (params (clutch :type Float%20%28double-precision%29))
  ;[0.02062 0.15 0.03603 0.5] Controls
  (bind _asbp_driving_seat (Utilities|Casting|CastToBP_DrivingSeat (Variables|/Script/Engine.ChildActorComponent|GetChildActor (Variables|Default|GetBP_DrivingSeat))))
  (Default|AnimateClutch _asbp_driving_seat clutch))

(event Custom|SR_Spawn_Occupant
  ;[1 0.6806 0.08897] SR_SpawnOwningPlayer
  (bind _asbp_cgmb_carla_vr (Utilities|Casting|CastToBP_CGMB_CarlaVR (Game|GetGameMode)))
  (Variables|/Game/Carla/CarlaVR/VR_Framework/BP_CGMB_CarlaVR.BP_CGMB_CarlaVR_C|SetTargetVehicle _asbp_cgmb_carla_vr self)
  (Utilities|FlowControl|Delay 3.0)
  (Default|SetPlayerOnboard _asbp_cgmb_carla_vr))

(event Custom|Set_Custom_Steering
  (params (Steering :type Float%20%28double-precision%29))
  ;[0.02062 0.15 0.03603 0.5] Controls
  (Class|ChaosVehicleMovementComponent|SetSteeringInput (Variables|Default|GetVehicleMovementComponent) Steering)
  (bind _asbp_driving_seat (Utilities|Casting|CastToBP_DrivingSeat (Variables|/Script/Engine.ChildActorComponent|GetChildActor (Variables|Default|GetBP_DrivingSeat))))
  (Default|AnimateSW _asbp_driving_seat (- Steering (Variables|Default|GetPreviousSteering)))
  (Variables|Default|SetPreviousSteering Steering))

(event Custom|Set_Custom_Brake
  (params (Brake :type Float%20%28double-precision%29))
  ;[0.02062 0.15 0.03603 0.5] Controls
  (Class|ChaosVehicleMovementComponent|SetBrakeInput (Variables|Default|GetVehicleMovementComponent) Brake)
  (bind _asbp_driving_seat (Utilities|Casting|CastToBP_DrivingSeat (Variables|/Script/Engine.ChildActorComponent|GetChildActor (Variables|Default|GetBP_DrivingSeat))))
  (Default|AnimateBrake _asbp_driving_seat Brake))

(event Custom|Set_Custom_HandBrake
  (params (HandBrake :type Boolean))
  ;[0.02062 0.15 0.03603 0.5] Controls
  (Class|ChaosVehicleMovementComponent|SetHandbrakeInput (Variables|Default|GetVehicleMovementComponent) HandBrake))

(event Custom|Set_Custom_Gear
  (params (Gear :type Integer))
  ;[0.02062 0.15 0.03603 0.5] Controls
  (bind _output_get (Variables|Default|Setforced_Gear Gear))
  (bind _asbp_driving_seat (Utilities|Casting|CastToBP_DrivingSeat (Variables|/Script/Engine.ChildActorComponent|GetChildActor (Variables|Default|GetBP_DrivingSeat))))
  (if (== _output_get -1)
    (Default|AnimateGear _asbp_driving_seat 6)
    (else
      (Default|AnimateGear _asbp_driving_seat _output_get))))

(event Custom|JoystickSubsystemReady
  ;[0.01554 0.1455 0.15 0.5] Setting up joystick plugin
  (Development|PrintString "Joystick subsystem is ready" true true "(R=0.000000,G=0.966856,B=1.000000,A=1.000000)" 5.0))

(event Custom|JoystickUnplugged
  (params (InstanceId :type Joystick%20Instance%20Id%20Structure%20%28by%20ref%29))
  ;[0.01554 0.1455 0.15 0.5] Setting up joystick plugin
)

(event Custom|JoystickPluggedIn
  (params (InstanceId :type Joystick%20Instance%20Id%20Structure%20%28by%20ref%29))
  ;[0.01554 0.1455 0.15 0.5] Setting up joystick plugin
)

(event EventBeginPlay
  (bind _returnvalue (|JoystickSubsystem))
  ;[0.007529 0.09962 0.15 0.5] SetUp Vehicle
  (|CallParentFunction)
  (CallFunction|SRSpawnOccupant)
  (bind _aswb_speedometer (Utilities|Casting|CastToWB_Speedometer (UserInterface|GetUserWidgetObject (Variables|Default|GetW_Speedometer))))
  (Default|SetParentVehicle _aswb_speedometer self)
  (bind _aswb_rpm (Utilities|Casting|CastToWB_RPM (UserInterface|GetUserWidgetObject (Variables|Default|GetW_RPM))))
  (Default|SetParentVehicle _aswb_rpm self)
  (bind _aschaos_wheeled_vehicle_movement_component (Utilities|Casting|CastToChaosWheeledVehicleMovementComponent (Variables|Default|GetVehicleMovementComponent)))
  ;[0.01554 0.1455 0.15 0.5] Setting up joystick plugin
  (EventDispatchers|AssignJoystickSubsystemReady _returnvalue (delegate Custom|JoystickSubsystemReady))
  (EventDispatchers|BindEventtoJoystickPluggedinDelegate _returnvalue (delegate Custom|JoystickPluggedIn))
  (EventDispatchers|BindEventtoJoystickUnpluggedDelegate _returnvalue (delegate Custom|JoystickUnplugged))
  (Variables|Default|SetDeviceID (Utilities|Array|Get(acopy) (Class|JoystickSubsystem|GetInstanceIds _returnvalue)))
  (bind _returnvalue_2 (Game|ConstructObjectfromClass "/Game/Carla/CarlaVR/VR_Framework/Avatar/Input/FF_Condition_Steering.FF_Condition_Steering_C" (Variables|Default|GetDeviceID)))
  (Variables|Default|SetFFB_Effect _returnvalue_2))

(event EventTick
  (params (DeltaSeconds :type Float%20%28single-precision%29))
  (bind _a_wind (Variables|Default|GetA_Wind))
  ;[0.15 0.15 0.15 0.5] ForcingManualTransmission
  (bind _aschaos_wheeled_vehicle_movement_component (Utilities|Casting|CastToChaosWheeledVehicleMovementComponent (Variables|Default|GetVehicleMovementComponent)))
  (Audio|Parameter|SetFloatParameter (Variables|Default|GetA_Engine) "RPM" (Variables|Default|GetEngineSoundDrive) :!class /Script/Engine.AudioComponent)
  (Audio|Parameter|SetFloatParameter _a_wind "Speed" (/ (Vehicle|GetForwardSpeed _aschaos_wheeled_vehicle_movement_component) 1e+02) :!class /Script/AudioExtensions.AudioParameterControllerInterface)
  (Audio|Components|Audio|SetVolumeMultiplier _a_wind (/ (Vehicle|GetForwardSpeed _aschaos_wheeled_vehicle_movement_component) 1e+02) :!class /Script/Engine.AudioComponent))

(fn ConstructionScript
  (|CallParentFunction))

(fn FindButtonLocation
  (params (NewParam :type BP%20Driving%20Seat%20Object%20Reference))
  (bind _asbp_driving_seat (Utilities|Casting|CastToBP_DrivingSeat (Variables|/Script/Engine.ChildActorComponent|GetChildActor (Variables|Default|GetBP_DrivingSeat))))
  (bind (_button_l _button_b) (Default|GetButtonPosition _asbp_driving_seat))
  (return _button_l _button_b))

(fn GetFront
  (return (Variables|/Script/Engine.ChildActorComponent|GetChildActor (Variables|Default|GetBP_VC_start))))