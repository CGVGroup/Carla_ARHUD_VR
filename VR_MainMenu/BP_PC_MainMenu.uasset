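; Main menu PlayerController that picks a VR or desktop pawn for the player at startup.
; BeginPlay enables HMD and, based on headset connection and local control, calls SR spawn events that delegate to BP_GM_MainMenu.
; Debug-style hotkeys select scenario and HUD/HDD Vivace vehicle, then open Mappano or Matrix through the launch menu on BP_MainMenu_Actor's widget.
; An unconnected branch holds unused menu-spawning logic for VR and viewport.
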(event Custom|SR_SpawnPlayer_VR
  ;[1 0.4745 0.07292] SR_SpawnPlayer
  (bind _asbp_gm_main_menu (Utilities|Casting|CastToBP_GM_MainMenu (Game|GetGameMode)))
  (Default|SpawnPawnVR _asbp_gm_main_menu self))

(event Custom|SR_Spawn_Player_Desktop
  ;[0.4583 0.2464 0.04143 0.5] SR_SapwnDesktop
  (bind _asbp_gm_main_menu (Utilities|Casting|CastToBP_GM_MainMenu (Game|GetGameMode)))
  (Default|SpawnPawnDesktop _asbp_gm_main_menu)
  (Variables|Default|SetbShowMouseCursor self true))

(event EventBeginPlay
  (Development|PrintString "pc says hello")
  (Class|HeadMountedDisplayFunctionLibrary|EnableHMD true)
  ;[0.15 0.15 0.15 0.5] Make dual boot in single build -> use to determine folder name
  (if (and (Class|HeadMountedDisplayFunctionLibrary|IsHeadMountedDisplayConnected) (Pawn|IsLocalPlayerController))
    (CallFunction|SRSpawnPlayerVR)
    (else
      (CallFunction|SRSpawnPlayerDesktop))))

(event Input|KeyboardEvents|L
  (params (Key :type Key%20Structure :default "None"))
  (:Pressed
    (bind _returnvalue (Actor|GetActorOfClass "/Game/Carla/CarlaVR/VR_MainMenu/Widgets/BP_MainMenu_Actor.BP_MainMenu_Actor_C"))
    (bind _aswb_main_menu_master (Utilities|Casting|CastToWB_MainMenu_Master (UserInterface|GetWidget (Variables|/Game/Carla/CarlaVR/VR_MainMenu/Widgets/BP_MainMenu_Actor.BP_MainMenu_Actor_C|GetWidget _returnvalue))))
    (Default|OpenMappano (Variables|/Game/Carla/CarlaVR/VR_MainMenu/Widgets/WB_MainMenu_Master.WB_MainMenu_Master_C|GetWB_LaunchMenu _aswb_main_menu_master))))

(event Input|KeyboardEvents|Ò
  (params (Key :type Key%20Structure :default "None"))
  (:Pressed
    (bind _returnvalue (Actor|GetActorOfClass "/Game/Carla/CarlaVR/VR_MainMenu/Widgets/BP_MainMenu_Actor.BP_MainMenu_Actor_C"))
    (bind _aswb_main_menu_master (Utilities|Casting|CastToWB_MainMenu_Master (UserInterface|GetWidget (Variables|/Game/Carla/CarlaVR/VR_MainMenu/Widgets/BP_MainMenu_Actor.BP_MainMenu_Actor_C|GetWidget _returnvalue))))
    (Default|OpenMatrix (Variables|/Game/Carla/CarlaVR/VR_MainMenu/Widgets/WB_MainMenu_Master.WB_MainMenu_Master_C|GetWB_LaunchMenu _aswb_main_menu_master) (Variables|Default|Getvehicle) (Variables|Default|Getscenario))))

(event Input|KeyboardEvents|3
  (params (Key :type Key%20Structure :default "None"))
  (:Pressed
    (Variables|Default|Setscenario "1")
    (Variables|Default|Setvehicle "BP_HDD_Vivace")))

(event Input|KeyboardEvents|1
  (params (Key :type Key%20Structure :default "None"))
  (:Pressed
    (Variables|Default|Setscenario "1")
    (Variables|Default|Setvehicle "BP_HUD_Vivace")))

(event Input|KeyboardEvents|2
  (params (Key :type Key%20Structure :default "None"))
  (:Pressed
    (Variables|Default|Setscenario "2")
    (Variables|Default|Setvehicle "BP_HUD_Vivace")))

(event Input|KeyboardEvents|4
  (params (Key :type Key%20Structure :default "None"))
  (:Pressed
    (Variables|Default|Setscenario "2")
    (Variables|Default|Setvehicle "BP_HDD_Vivace")))

(fn ConstructionScript)