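; Main menu game mode that provides separate setup functions for VR and desktop players.
; The VR function destroys the controller's current pawn, possesses the VR pawn already in the level and spawns a menu actor positioned relative to its camera.
; The desktop function applies windowed resolution settings and adds the master menu widget to the viewport.
; BeginPlay is empty, and the branch that spawns a new VR pawn is disconnected.
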(event EventBeginPlay)

(fn ConstructionScript)

(fn SpawnPawnVR
  (params (PC :type Player%20Controller%20Object%20Reference))
  (bind _returnvalue (Pawn|GetControlledPawn PC))
  (Utilities|IsValid _returnvalue
    (:Is%20Valid
      (Actor|DestroyActor _returnvalue))
    (:Is%20Not%20Valid
      _))
  (bind _returnvalue_2 (Actor|GetActorOfClass "/Game/Carla/CarlaVR/VR_Framework/Avatar/BP_P_VRPawn_Controller.BP_P_VRPawn_Controller_C"))
  (bind _output_get (Variables|Default|SetVRPawn_C _returnvalue_2))
  (Pawn|Possess PC _output_get)
  (Development|PrintString "Spawn VRPawn" true true "(R=1.000000,G=0.007625,B=0.653255,A=1.000000)" 25.0)
  (Game|SpawnActorfromClass "/Game/Carla/CarlaVR/VR_MainMenu/Widgets/BP_MainMenu_Actor.BP_MainMenu_Actor_C" (Math|Transform|MakeTransform (+ (* (Math|Vector|GetForwardVector (Variables|/Game/Carla/CarlaVR/VR_Framework/Avatar/BP_P_VRPawn_Controller.BP_P_VRPawn_Controller_C|GetCamera (Variables|Default|GetVRPawn_C))) -6e+01) (.location (Transformation|GetWorldTransform (Variables|/Game/Carla/CarlaVR/VR_Framework/Avatar/BP_P_VRPawn_Controller.BP_P_VRPawn_Controller_C|GetCamera (Variables|Default|GetVRPawn_C))))) (Math|Rotator|CombineRotators (.rotation (Transformation|GetWorldTransform (Variables|/Game/Carla/CarlaVR/VR_Framework/Avatar/BP_P_VRPawn_Controller.BP_P_VRPawn_Controller_C|GetCamera (Variables|Default|GetVRPawn_C)))) "0.000000,180.000000,0.000000") (.scale (Transformation|GetWorldTransform (Variables|/Game/Carla/CarlaVR/VR_Framework/Avatar/BP_P_VRPawn_Controller.BP_P_VRPawn_Controller_C|GetCamera (Variables|Default|GetVRPawn_C))))) "Undefined" "MultiplyWithRoot" 0 0)
  (return))

(fn SpawnPawnDesktop
  (bind _returnvalue (Settings|GetGameUserSettings))
  (Class|GameUserSettings|SetFullscreenMode _returnvalue "Windowed")
  (Class|GameUserSettings|SetScreenResolution _returnvalue (Variables|Default|GetResolution))
  (Class|GameUserSettings|ApplySettings _returnvalue false)
  (Development|PrintString "Desktop Mode")
  (bind _returnvalue_2 (UserInterface|CreateWidget "/Game/Carla/CarlaVR/VR_MainMenu/Widgets/WB_MainMenu_Master.WB_MainMenu_Master_C" (Game|GetPlayerController 0)))
  (UserInterface|Viewport|AddtoViewport _returnvalue_2 0)
  (Default|SetIDType _returnvalue_2 false))